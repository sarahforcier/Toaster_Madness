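; Player-controlled toaster actor that launches a physics toast: holding the shoot input while hovering charges a timeline, and release replaces the previous toast with one fired along the toaster's up axis.
; Charge sets toast speed and drives progress bars and hand animation, while the eyes track the live toast.
; In the game mode's edit mode, gated Tick logic lets cursor traces drag the body and rotate it via a sphere handle in the YZ plane.
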(event OnClicked(Toaster_child_visible)
  (params (TouchedComponent :type Primitive%20Component%20Object%20Reference) (ButtonPressed :type Key%20Structure))
  (bind _returnvalue (Game|GetPlayerController 0))
  (bind (_hitresult _returnvalue_2) (Game|Player|GetHitResultUnderCursorbyChannel _returnvalue "TraceTypeQuery1" true))
  ;[1 1 1] Move toaster by using mouse click and drag. (Make sure its collision component visibility channel is not marked as "ignored")
  (Utilities|FlowControl|Gate true) ; enters at Open
)

(event OnClicked(Sphere)
  (params (TouchedComponent :type Primitive%20Component%20Object%20Reference) (ButtonPressed :type Key%20Structure))
  (bind _returnvalue (Game|GetPlayerController 0))
  (bind _defaultsceneroot (Variables|Default|GetDefaultSceneRoot))
  (bind _returnvalue_2 (Transformation|GetWorldTransform _defaultsceneroot))
  (bind (_hitresult _returnvalue_3) (Game|Player|GetHitResultUnderCursorbyChannel _returnvalue "TraceTypeQuery1" true))
  (bind _returnvalue_4 (Math|Transform|InvertTransform _returnvalue_2))
  (bind _location (Collision|BreakHitResult _hitresult))
  (bind _returnvalue_5 (* _location "0.000000,1.000000,1.000000"))
  (bind _returnvalue_6 (Math|Transform|TransformLocation _returnvalue_4 _returnvalue_5))
  (bind (_x _y _z) (Math|Vector|BreakVector _returnvalue_6))
  ;[1 1 1] Move toaster by using mouse click and drag. (Make sure its collision component visibility channel is not marked as "ignored")
  (Utilities|FlowControl|Gate true) ; enters at Open
)

(event OnReleased(Sphere)
  (params (TouchedComponent :type Primitive%20Component%20Object%20Reference) (ButtonReleased :type Key%20Structure))
  (bind _returnvalue (Game|GetPlayerController 0))
  (bind _defaultsceneroot (Variables|Default|GetDefaultSceneRoot))
  (bind _returnvalue_2 (Transformation|GetWorldTransform _defaultsceneroot))
  (bind (_hitresult _returnvalue_3) (Game|Player|GetHitResultUnderCursorbyChannel _returnvalue "TraceTypeQuery1" true))
  (bind _returnvalue_4 (Math|Transform|InvertTransform _returnvalue_2))
  (bind _location (Collision|BreakHitResult _hitresult))
  (bind _returnvalue_5 (* _location "0.000000,1.000000,1.000000"))
  (bind _returnvalue_6 (Math|Transform|TransformLocation _returnvalue_4 _returnvalue_5))
  (bind (_x _y _z) (Math|Vector|BreakVector _returnvalue_6))
  ;[1 1 1] Move toaster by using mouse click and drag. (Make sure its collision component visibility channel is not marked as "ignored")
  (Utilities|FlowControl|Gate true) ; enters at Close
)

(event OnReleased(Toaster_child_visible)
  (params (TouchedComponent :type Primitive%20Component%20Object%20Reference) (ButtonReleased :type Key%20Structure))
  (bind _returnvalue (Game|GetPlayerController 0))
  (bind (_hitresult _returnvalue_2) (Game|Player|GetHitResultUnderCursorbyChannel _returnvalue "TraceTypeQuery1" true))
  ;[1 1 1] Move toaster by using mouse click and drag. (Make sure its collision component visibility channel is not marked as "ignored")
  (Utilities|FlowControl|Gate true) ; enters at Close
)

(event OnBeginCursorOver(Toaster_child_visible)
  (params (TouchedComponent :type Primitive%20Component%20Object%20Reference))
  ;[1 1 1] Shoot toast with left mouse key
  (Variables|Default|SetIsHovering true))

(event OnEndCursorOver(Toaster_child_visible)
  (params (TouchedComponent :type Primitive%20Component%20Object%20Reference))
  ;[1 1 1] Shoot toast with left mouse key
  (Variables|Default|SetIsHovering false))

(event EventBeginPlay
  ;[1 1 1] Allow for input on player controller
  (Input|EnableInput (Game|GetPlayerController 0)))

(event Collision|EventActorBeginOverlap
  (params (OtherActor :type Actor%20Object%20Reference)))

(event EventTick
  (params (DeltaSeconds :type Float%20%28single-precision%29))
  (bind _returnvalue (Game|GetPlayerController 0))
  (bind _righteyebase (Variables|Default|GetRightEyeBase))
  (bind _toasty (Variables|Default|GetToasty))
  (bind _defaultsceneroot (Variables|Default|GetDefaultSceneRoot))
  (bind _toasty_2 (Variables|Default|GetToasty))
  (bind _lefteyebase (Variables|Default|GetLeftEyeBase))
  (bind _defaultsceneroot_2 (Variables|Default|GetDefaultSceneRoot))
  (bind _handscontainer (Variables|Default|GetHandsContainer))
  (bind _torus (Variables|Default|GetTorus))
  (bind _returnvalue_2 (Transformation|GetWorldTransform _defaultsceneroot))
  (bind _returnvalue_3 (Transformation|GetWorldLocation _righteyebase))
  (bind _returnvalue_4 (Transformation|GetWorldLocation _lefteyebase))
  (bind (_hitresult _returnvalue_5) (Game|Player|GetHitResultUnderCursorbyChannel _returnvalue "TraceTypeQuery1" true))
  (bind _toastposition (Variables|/Game/GameObjects/ToastBP.ToastBP_C|GetToastPosition _toasty_2))
  (bind _returnvalue_6 (Math|Transform|InvertTransform _returnvalue_2))
  (bind _returnvalue_7 (- _toastposition _returnvalue_3))
  (bind _returnvalue_8 (- _toastposition _returnvalue_4))
  (bind _location (Collision|BreakHitResult _hitresult))
  (bind _returnvalue_9 (Math|Vector|Normalize _returnvalue_7))
  (bind _returnvalue_10 (Math|Vector|Normalize _returnvalue_8))
  (bind _returnvalue_11 (* _location "0.000000,1.000000,1.000000"))
  (bind _returnvalue_12 (Math|Transform|TransformLocation _returnvalue_6 _returnvalue_11))
  (bind (_x _y _z) (Math|Vector|BreakVector _returnvalue_9))
  (bind (_x_2 _y_2 _z_2) (Math|Vector|BreakVector _returnvalue_10))
  (bind (_x_3 _y_3 _z_3) (Math|Vector|BreakVector _returnvalue_12))
  (Utilities|FlowControl|Sequence
    (:then_0
      (Utilities|FlowControl|Sequence
        (:then_0
          ;[1 1 1] Move toaster by using mouse click and drag. (Make sure its collision component visibility channel is not marked as "ignored")
          (Utilities|FlowControl|Sequence
            (:then_0
              (Utilities|FlowControl|Gate true
                (:Exit
                  (bind _asmouse_mvmt_tests_3_game_mode (Utilities|Casting|CastToMouseMvmtTests_3_GameMode (Game|GetGameMode)))
                  (if (and (Variables|/Game/MouseMvmtTests_3_GameMode.MouseMvmtTests_3_GameMode_C|GetIsEditMode _asmouse_mvmt_tests_3_game_mode) _returnvalue_5)
                    (Transformation|SetRelativeLocation _defaultsceneroot_2 _returnvalue_11 false false)))))
            (:then_1
              (Utilities|FlowControl|Gate true
                (:Exit
                  (bind _asmouse_mvmt_tests_3_game_mode_2 (Utilities|Casting|CastToMouseMvmtTests_3_GameMode (Game|GetGameMode)))
                  (if (and (Variables|/Game/MouseMvmtTests_3_GameMode.MouseMvmtTests_3_GameMode_C|GetIsEditMode _asmouse_mvmt_tests_3_game_mode_2) _returnvalue_5)
                    (Transformation|AddRelativeRotation _defaultsceneroot_2 (Math|Vector|RotatorfromAxisandAngle "1.000000, 0, 0" (Math|Trig|Atan2(Radians) _z_3 _y_3)) false false)))))
            (:then_2
              (bind _asmouse_mvmt_tests_3_game_mode_3 (Utilities|Casting|CastToMouseMvmtTests_3_GameMode (Game|GetGameMode)))
              (if (Variables|/Game/MouseMvmtTests_3_GameMode.MouseMvmtTests_3_GameMode_C|GetIsEditMode _asmouse_mvmt_tests_3_game_mode_3)
                (Rendering|SetVisibility _torus true true)
                (if (Utilities|IsValid _toasty)
                  (Actor|DestroyActor _toasty))
                (else
                  (Rendering|SetVisibility _torus false true))))))
        (:then_1
          ;[1 1 1] Shoot toast with left mouse key
          (bind _asmouse_mvmt_tests_3_game_mode_4 (Utilities|Casting|CastToMouseMvmtTests_3_GameMode (Game|GetGameMode)))
          (Utilities|FlowControl|Sequence
            (:then_0
              (Rendering|SetVisibility (Variables|Default|Getprogbar_1) (and (> (Math|Float|MapRangeClamped (stale Input|ActionEvents|InputActionShootToast _speed) 0.0 2.0 0.0 1.0) 0.0) (and (Variables|Default|GetIsPressing) (not (Variables|/Game/MouseMvmtTests_3_GameMode.MouseMvmtTests_3_GameMode_C|GetIsEditMode _asmouse_mvmt_tests_3_game_mode_4)))) false)
              (Rendering|SetVisibility (Variables|Default|Getprogbar_2) (and (>= (Math|Float|MapRangeClamped (stale Input|ActionEvents|InputActionShootToast _speed) 0.0 2.0 0.0 1.0) 0.2) (and (Variables|Default|GetIsPressing) (not (Variables|/Game/MouseMvmtTests_3_GameMode.MouseMvmtTests_3_GameMode_C|GetIsEditMode _asmouse_mvmt_tests_3_game_mode_4)))) false)
              (Rendering|SetVisibility (Variables|Default|Getprogbar_3) (and (>= (Math|Float|MapRangeClamped (stale Input|ActionEvents|InputActionShootToast _speed) 0.0 2.0 0.0 1.0) 0.4) (and (Variables|Default|GetIsPressing) (not (Variables|/Game/MouseMvmtTests_3_GameMode.MouseMvmtTests_3_GameMode_C|GetIsEditMode _asmouse_mvmt_tests_3_game_mode_4)))) false)
              (Rendering|SetVisibility (Variables|Default|Getprogbar_4) (and (>= (Math|Float|MapRangeClamped (stale Input|ActionEvents|InputActionShootToast _speed) 0.0 2.0 0.0 1.0) 0.6) (and (Variables|Default|GetIsPressing) (not (Variables|/Game/MouseMvmtTests_3_GameMode.MouseMvmtTests_3_GameMode_C|GetIsEditMode _asmouse_mvmt_tests_3_game_mode_4)))) false)
              (Rendering|SetVisibility (Variables|Default|Getprogbar_5) (and (>= (Math|Float|MapRangeClamped (stale Input|ActionEvents|InputActionShootToast _speed) 0.0 2.0 0.0 1.0) 0.8) (and (Variables|Default|GetIsPressing) (not (Variables|/Game/MouseMvmtTests_3_GameMode.MouseMvmtTests_3_GameMode_C|GetIsEditMode _asmouse_mvmt_tests_3_game_mode_4)))) false))
            (:then_1
              ;[1 1 1] Hand animation
              (if (and (Variables|Default|GetIsPressing) (not (Variables|/Game/MouseMvmtTests_3_GameMode.MouseMvmtTests_3_GameMode_C|GetIsEditMode _asmouse_mvmt_tests_3_game_mode_4)))
                (Transformation|SetRelativeTransform _handscontainer (Math|Transform|MakeTransform (Math|Vector|MakeVector 0.0 0.0 (* (Math|Float|MapRangeClamped (stale Input|ActionEvents|InputActionShootToast _speed) 0.0 2.0 0.0 1.0) -4e+01)) "0, 0, 0" "1,1.000000,1") false false)
                (else
                  (Transformation|SetRelativeTransform _handscontainer (Math|Transform|MakeTransform "0, 0, 0") false false))))))))
    (:then_1
      (if (Utilities|IsValid _toasty_2)
        (Utilities|FlowControl|Sequence
          (:then_0
            (Transformation|SetRelativeTransform _lefteyebase (Math|Transform|MakeTransform (Variables|/Script/Engine.SceneComponent|GetRelativeLocation _lefteyebase) (Math|Rotator|MakeRotator (Class|KismetMathLibrary|DegAtan2 _y_2 _z_2) 0.0 0.0) "1.000000,1.000000,1") false false))
          (:then_1
            (Transformation|SetRelativeTransform _righteyebase (Math|Transform|MakeTransform (Variables|/Script/Engine.SceneComponent|GetRelativeLocation _righteyebase) (Math|Rotator|MakeRotator (Class|KismetMathLibrary|DegAtan2 _y _z) 0.0 0.0)) false false)))))))

(event Input|ActionEvents|InputActionShootToast
  (params (Key :type Key%20Structure))
  (bind _returnvalue (Math|Transform|MakeTransform "0, 0, 0"))
  (bind _defaultsceneroot (Variables|Default|GetDefaultSceneRoot))
  (bind _returnvalue_2 (Transformation|GetWorldTransform _defaultsceneroot))
  (bind _returnvalue_3 (Math|Transform|ComposeTransforms _returnvalue _returnvalue_2))
  ;[1 1 1] Shoot toast with left mouse key
  (:Pressed
    (Utilities|FlowControl|Sequence
      (:then_0
        (if (Variables|Default|GetIsHovering)
          (bind _asmouse_mvmt_tests_3_game_mode (Utilities|Casting|CastToMouseMvmtTests_3_GameMode (Game|GetGameMode)))
          (if (not (Variables|/Game/MouseMvmtTests_3_GameMode.MouseMvmtTests_3_GameMode_C|GetIsEditMode _asmouse_mvmt_tests_3_game_mode))
            (bind _speed (Timeline|ShootTimeline PlayFromStart)))))
      (:then_1
        (Variables|Default|SetIsPressing true))))
  (:Released
    (Utilities|FlowControl|Sequence
      (:then_0
        (if (Variables|Default|GetIsHovering)
          (bind _asmouse_mvmt_tests_3_game_mode_2 (Utilities|Casting|CastToMouseMvmtTests_3_GameMode (Game|GetGameMode)))
          (if (not (Variables|/Game/MouseMvmtTests_3_GameMode.MouseMvmtTests_3_GameMode_C|GetIsEditMode _asmouse_mvmt_tests_3_game_mode_2))
            (if (Utilities|IsValid (Variables|Default|GetToasty))
              (Actor|DestroyActor (Variables|Default|GetToasty)))
            (bind _returnvalue_4 (Game|SpawnActorfromClass "/Game/GameObjects/ToastBP.ToastBP_C" _returnvalue_3 "Undefined" 0 0))
            (bind _output_get (Variables|Default|SetToasty _returnvalue_4))
            (Variables|/Game/GameObjects/ToastBP.ToastBP_C|SetToastSpeed _output_get (Math|Float|MapRangeClamped _speed 0.0 2.0 0.0 1.0)) ; Set the normalized force for the toast/ball relationship
            (Physics|SetPhysicsLinearVelocity (Variables|/Game/GameObjects/ToastBP.ToastBP_C|GetCube _output_get) (Math|Transform|TransformDirection _returnvalue_3 (Math|Vector|MakeVector 0.0 0.0 (Math|Float|Lerp 1.75e+03 2.5e+03 (Math|Float|MapRangeClamped _speed 0.0 2.0 0.0 1.0)))) false "None")
            (Audio|Components|Audio|Play (Variables|Default|GetToasterShootSound) 0.0)
            (Timeline|ShootTimeline Stop))))
      (:then_1
        (Variables|Default|SetIsPressing false)))))

(fn ConstructionScript)