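; StarBP is a collectible star that spins in place and is picked up by the falling toast (FallingBallBP).
; Tick rotates the root by a fixed step per frame, so spin speed depends on frame rate.
; On overlap with the toast, it increments NumCollected on the first StarsBP actor found and hides the Star component.
; The actor is not destroyed or disabled, so repeat overlaps count again.
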(event EventBeginPlay)

(event Collision|EventActorBeginOverlap
  (params (OtherActor :type Actor%20Object%20Reference))
  ;[1 1 1] Increment stars collected if hit by toast
  (Utilities|Casting|CastToFallingBallBP OtherActor)
  (bind _outactors (Actor|GetAllActorsOfClass "/Game/GameObjects/StarsBP.StarsBP_C"))
  (Variables|/Game/GameObjects/StarsBP.StarsBP_C|SetnumCollected (Utilities|Array|Get(acopy) _outactors) (+ (Variables|/Game/GameObjects/StarsBP.StarsBP_C|GetnumCollected (Utilities|Array|Get(acopy) _outactors)) 1))
  (Rendering|SetVisibility (Variables|Default|GetStar) false false))

(event EventTick
  (params (DeltaSeconds :type Float%20%28single-precision%29))
  (Transformation|AddLocalRotation (Variables|Default|GetDefaultSceneRoot) "0.000000,0.000000,2.000000" false false))

(fn ConstructionScript)