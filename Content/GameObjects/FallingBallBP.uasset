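; Physics ball Blueprint that falls through a level, bounces off toast and returns to its start point on reset.
; Tick triggers the shared reset while the game mode is in edit mode or when the ball drops below a Z threshold.
; The reset zeroes velocity, restores position, re-shows stars and clears the collected count.
; Hitting a ToastBP keeps the travel direction but sets speed by interpolating on that toast's ToastSpeed.
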(event EventBeginPlay
  ;[1 1 1] Base falling ball logic
  (Variables|Default|SetFallingBallInitialPosition (Transformation|GetActorLocation)))

(event Collision|EventActorBeginOverlap
  (params (OtherActor :type Actor%20Object%20Reference)))

(event EventTick
  (params (DeltaSeconds :type Float%20%28single-precision%29))
  ;[1 1 1] Base falling ball logic
  (Utilities|FlowControl|Sequence
    (:then_0
      (bind _asmouse_mvmt_tests_3_game_mode (Utilities|Casting|CastToMouseMvmtTests_3_GameMode (Game|GetGameMode)))
      (if (Variables|/Game/MouseMvmtTests_3_GameMode.MouseMvmtTests_3_GameMode_C|GetIsEditMode _asmouse_mvmt_tests_3_game_mode)
        (for _array_element (stale _outactors_2) :!label _label
          (Rendering|SetVisibility (Variables|/Game/GameObjects/StarBP.StarBP_C|GetStar _array_element) true false))
        (bind _outactors (Actor|GetAllActorsOfClass "/Game/GameObjects/StarsBP.StarsBP_C"))
        (Variables|/Game/GameObjects/StarsBP.StarsBP_C|SetnumCollected (Utilities|Array|Get(acopy) _outactors) 0)
        (Transformation|SetActorLocation self (Variables|Default|GetFallingBallInitialPosition) false false)
        (Physics|SetPhysicsLinearVelocity (Variables|Default|GetSphere) "0, 0, 0" false "None")))
    (:then_1
      (if (> -4e+02 (.Z (Math|Vector|BreakVector (Transformation|GetActorLocation))))
        (bind _outactors_2 (Actor|GetAllActorsOfClass "/Game/GameObjects/StarBP.StarBP_C"))
        (goto _label)))))

(event Collision|EventHit
  (params (MyComp :type Primitive%20Component%20Object%20Reference) (Other :type Actor%20Object%20Reference) (OtherComp :type Primitive%20Component%20Object%20Reference) (bSelfMoved :type Boolean) (HitLocation :type Vector :default "0, 0, 0") (HitNormal :type Vector :default "0, 0, 0") (NormalImpulse :type Vector :default "0, 0, 0") (Hit :type Hit%20Result%20Structure%20%28by%20ref%29))
  (bind _astoast_bp (Utilities|Casting|CastToToastBP Other))
  (bind _returnvalue (Physics|GetPhysicsLinearVelocity (Variables|Default|GetSphere) "None"))
  (Physics|SetPhysicsLinearVelocity (Variables|Default|GetSphere) (* (Math|Vector|Normalize _returnvalue) (Math|Float|Lerp 1.2e+03 2.5e+03 (Variables|/Game/GameObjects/ToastBP.ToastBP_C|GetToastSpeed _astoast_bp))) false "None"))

(fn ConstructionScript)